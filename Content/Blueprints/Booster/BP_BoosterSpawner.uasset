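; Booster spawner actor that periodically spawns BP_BoosterMaster pickups from a box volume.
; On the authority only, a looping timer at SpawnRate spawns a scaled-down, rotated booster, passing along its BPBooster variable.
; Spawn position adds GetRandomLocation to the box's location, though that function's random-range nodes appear unconnected.
; The construction script sizes the box's X extent from BoxExtendX.
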(event Custom|SpawnBooster
  (Game|SpawnActorfromClass "/Game/Blueprints/Booster/BP_BoosterMaster.BP_BoosterMaster_C" (Math|Transform|MakeTransform (+ (Transformation|GetWorldLocation (Variables|Default|GetBox)) (Utilities|GetRandomLocation)) "0,-90.000000, 0" "0.400000,0.400000,0.400000") "Undefined" self (Variables|Default|GetBP%20Booster) 0))

(event EventBeginPlay
  (Networking|SwitchHasAuthority
    (:Authority
      (Utilities|Time|SetTimerbyEvent (delegate Custom|SpawnBooster) (Variables|Default|GetSpawnRate) true))))

(fn ConstructionScript
  (bind _box (Variables|Default|GetBox))
  (Transformation|SetWorldScale3D _box (Math|Vector|MakeVector 1.0 1.0 1.0))
  (Components|Box|SetBoxExtent _box (Math|Vector|MakeVector (Variables|Default|GetBoxExtendX) 3e+01 3e+01) true))

(fn PrintOnce
  (params (Append :type String) (InString :type String))
  (Development|PrintString (Utilities|String|Append Append InString) true true "(R=0.000000,G=0.660000,B=1.000000,A=1.000000)" 0.0))