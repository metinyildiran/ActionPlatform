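; Base pickup booster that fires an overridable, empty OnPickUp event and destroys itself when a Character overlaps its mesh.
; On authority, BeginPlay async-loads a random BPBooster class, then re-rolls the index to set the ChildActor class, so the two may differ.
; After a delay, a HideAndShow timeline drives opacity on the dynamic material created in construction, then destroys the actor.
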(event OnComponentBeginOverlap(BoosterMesh)
  (params (OverlappedComponent :type Primitive%20Component%20Object%20Reference) (OtherActor :type Actor%20Object%20Reference) (OtherComp :type Primitive%20Component%20Object%20Reference) (OtherBodyIndex :type Integer) (bFromSweep :type Boolean) (SweepResult :type Hit%20Result%20Structure%20%28by%20ref%29))
  (bind _ascharacter (Utilities|Casting|CastToCharacter OtherActor))
  (CallFunction|OnPickUp _ascharacter)
  (CallFunction|Destroy))

(event Custom|OnPickUp
  (params (Character :type Character%20Object%20Reference)))

(event Custom|Destroy
  (Actor|DestroyActor))

(event Custom|SR_HideAndShow
  (bind _opacity (Timeline|HideAndShow PlayFromStart)
    (:Update
      (Rendering|Material|SetScalarParameterValue (Variables|Default|GetDynamicMaterial) "Opacity" _opacity :!class /Script/Engine.MaterialInstanceDynamic))
    (:Finished
      (Utilities|IsValid self
        (:Is%20Valid
          (CallFunction|Destroy))))))

(event EventBeginPlay
  (bind _bp_booster (Variables|Default|GetBP_Booster))
  (bind _returnvalue (Utilities|Array|Length _bp_booster))
  (bind _returnvalue_2 (- _returnvalue 1))
  (bind _returnvalue_3 (Math|Random|RandomIntegerinRange 0 _returnvalue_2))
  (bind _output (Utilities|Array|Get(acopy) _bp_booster _returnvalue_3))
  (Networking|SwitchHasAuthority
    (:Authority
      (Utilities|AsyncLoadClassAsset _output
        (:Completed
          (ChildActorComponent|SetChildActorClass (Variables|Default|GetChildActor) (Utilities|ResolveSoftReference _output))
          (Utilities|FlowControl|Delay 7.6)
          (CallFunction|SRHideandShow))))))

(fn ConstructionScript
  (bind _returnvalue (Rendering|Material|CreateDynamicMaterialInstance (Variables|Default|GetBoosterMesh) 0 "/Game/Blueprints/Booster/Materials/M_BoosterMaster.M_BoosterMaster" "None" :!class /Script/Engine.PrimitiveComponent))
  (bind _output_get (Variables|Default|SetDynamicMaterial _returnvalue))
  (Rendering|Material|SetVectorParameterValue _output_get "Emissive" "(R=10.000000,G=10.000000,B=10.000000,A=1.000000)" :!class /Script/Engine.MaterialInstanceDynamic)
  (Rendering|Material|SetScalarParameterValue _output_get "Opacity" 1.0 :!class /Script/Engine.MaterialInstanceDynamic))