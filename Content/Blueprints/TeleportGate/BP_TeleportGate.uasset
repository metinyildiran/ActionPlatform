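; Paired teleport gate that moves an overlapping Character to its TargetGate, facing a yaw derived from this gate's rotation.
; Overlap disables collision on both gates, and a valid target also triggers the teleport, darkens both gates' dynamic materials and starts a cooldown timer.
; A looping timer mirrors the remaining time on both gates' text counters, while the cooldown's expiry restores collision and blue color.
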(event OnComponentBeginOverlap(Gate)
  (params (OverlappedComponent :type Primitive%20Component%20Object%20Reference) (OtherActor :type Actor%20Object%20Reference) (OtherComp :type Primitive%20Component%20Object%20Reference) (OtherBodyIndex :type Integer) (bFromSweep :type Boolean) (SweepResult :type Hit%20Result%20Structure%20%28by%20ref%29))
  (bind _ascharacter (Utilities|Casting|CastToCharacter OtherActor))
  (Utilities|DisableGate)
  (bind _targetgate (Variables|Default|GetTargetGate)
    (:then
      (Transformation|Teleport _ascharacter (Transformation|GetWorldLocation (Variables|BP_TeleportGate_C|GetGate _targetgate)) (Math|Rotator|MakeRotator 0.0 0.0 (+ (.yaw (Transformation|GetActorRotation)) -9e+01)))
      (CallFunction|SetGateColor "(R=0.000000,G=0.000000,B=0.015000,A=1.000000)")
      (bind _returnvalue (Utilities|Time|SetTimerbyEvent (delegate Custom|EnableGateEvent) 15.0))
      (Variables|Default|SetTimerHandle _returnvalue)
      (bind _returnvalue_2 (Utilities|Time|SetTimerbyFunctionName 0 "SetCounter" 0.1 true))
      (Variables|Default|SetSetCounterTimerHandle _returnvalue_2)
      (Rendering|SetVisibility (Variables|Default|GetCounterText) true false)
      (Rendering|SetVisibility (Variables|BP_TeleportGate_C|GetCounterText (Variables|Default|GetTargetGate)) true false))
    (:else)))

(event Custom|EnableGateEvent
  (Utilities|EnableGate)
  (CallFunction|SetGateColor "(R=0.000000,G=0.000000,B=1.000000,A=1.000000)"))

(event Custom|SetCounter
  (bind _timerhandle (Variables|Default|GetTimerHandle))
  (bind _returnvalue (Utilities|Time|GetTimerRemainingTimebyHandle _timerhandle))
  (bind _returnvalue_2 (Utilities|Text|ToText(Float) _returnvalue "HalfToEven" false true 1 324 0 0))
  (if (!= _returnvalue -1.0)
    (Rendering|Components|TextRender|SetText (Variables|Default|GetCounterText) _returnvalue_2)
    (Rendering|Components|TextRender|SetText (Variables|BP_TeleportGate_C|GetCounterText (Variables|Default|GetTargetGate)) _returnvalue_2)
    (else
      (Rendering|SetVisibility (Variables|Default|GetCounterText) false false)
      (Rendering|SetVisibility (Variables|BP_TeleportGate_C|GetCounterText (Variables|Default|GetTargetGate)) false false)
      (Utilities|Time|ClearandInvalidateTimerbyHandle (Variables|Default|GetTimerHandle))
      (Utilities|Time|ClearandInvalidateTimerbyHandle (Variables|Default|GetSetCounterTimerHandle)))))

(fn ConstructionScript
  (bind _returnvalue (Rendering|Material|CreateDynamicMaterialInstance (Variables|Default|GetGate) 0 "/Game/Blueprints/TeleportGate/M_TeleportGate.M_TeleportGate" "None" :!class /Script/Engine.PrimitiveComponent))
  (bind _output_get (Variables|Default|SetGateMaterial _returnvalue))
  (Rendering|Material|SetVectorParameterValue _output_get "Color" "(R=0.000000,G=0.000000,B=1.000000,A=1.000000)" :!class /Script/Engine.MaterialInstanceDynamic)
  (Transformation|SetWorldRotation (Variables|Default|GetCounterText) "0, 0, 0" false false))

(fn SetGateColor
  (params (Color :type Linear%20Color%20Structure))
  (Rendering|Material|SetVectorParameterValue (Variables|Default|GetGateMaterial) "Color" Color :!class /Script/Engine.MaterialInstanceDynamic)
  (Rendering|Material|SetVectorParameterValue (Variables|BP_TeleportGate_C|GetGateMaterial (Variables|Default|GetTargetGate)) "Color" Color :!class /Script/Engine.MaterialInstanceDynamic))