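; Test AI spawner actor that, when enabled, spawns a set number of enemies on the authority at BeginPlay.
; Each spawn picks a random EnemyList entry (Grenade, Minigun, Arrow or Magic) and maps it to an index into parallel class and behavior tree arrays.
; SpawnAI async-loads the class, then spawns it at the box location plus GetRandomLocation, whose random-offset nodes appear unconnected.
; The construction script sizes the box from BoxExtendX.
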(event EventBeginPlay
  (bind _enemylist (Variables|Default|GetEnemyList))
  (bind _returnvalue (Utilities|Array|Length _enemylist))
  (if (Variables|Default|GetIsEnabled)
    (Networking|SwitchHasAuthority
      (:Authority
        (for _index (range 1 (Variables|Default|GetAICount))
          (if (!= _returnvalue 0)
            (switch Utilities|FlowControl|Switch|SwitchonEnum_EnemyAIList (Utilities|Array|Get(acopy) _enemylist (Math|Random|RandomIntegerinRange 0 (- _returnvalue 1)))
              (:NewEnumerator0
                (Utilities|SpawnAI))
              (:NewEnumerator1
                (Utilities|SpawnAI 1))
              (:NewEnumerator2
                (Utilities|SpawnAI 2))
              (:NewEnumerator3
                (Utilities|SpawnAI 3)))))))))

(fn ConstructionScript
  (bind _box (Variables|Default|GetBox))
  (Transformation|SetWorldScale3D _box (Math|Vector|MakeVector 1.0 1.0 1.0))
  (Components|Box|SetBoxExtent _box (Math|Vector|MakeVector (Variables|Default|GetBoxExtendX) 3e+01 3e+01) true))