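; Game instance Blueprint, judging by its GI_ name, that hosts and joins online multiplayer sessions for co-op and PvP play.
; HostSession creates a non-LAN session, then opens the co-op or PvP map as a listen server.
; If creation fails, it destroys the session and retries with no attempt limit.
; JoinServer joins a given search result, alongside older advanced-session create events, one deprecated and the PvP one marked TODO.
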(event Custom|CreateServer
  ;[1 1 1] Deprecated
  (|AdvancedSession 0 (Game|GetPlayerController 0) 100 0 false true false true true false false false true
    (:OnSuccess
      (Development|PrintString "Server Created")
      (Game|OpenLevel(byName) "CoopMap" true "?listen"))))

(event Custom|JoinServer
  (params (Session :type Blueprint%20Session%20Result%20Structure))
  (|JoinSession (Game|GetPlayerController 0) Session))

(event Custom|CreatePVPServer
  ;[1 0.1971 0.7922] TODO PvP Level
  (|AdvancedSession 0 (Game|GetPlayerController 0) 100 0 false true false true true false false false true
    (:OnSuccess
      (Development|PrintString "PvP Server Created")
      (Game|OpenLevel(byName) "PVP_Map" true "?listen"))))

(event Custom|HostSession
  (params (Coop? :type Boolean))
  (if Coop? :!label _label
    (|Session (Game|GetPlayerController 0) 10 false
      (:OnSuccess
        (Development|PrintString "Coop Server Created Successfully")
        (Game|OpenLevel(byName) "CoopMap1" true "?listen"))
      (:OnFailure
        (|DestroySession (Game|GetPlayerController 0)
          (:OnSuccess
            (goto _label)))))
    (else
      (|Session (Game|GetPlayerController 0) 10 false :!label _label_2
        (:OnSuccess
          (Development|PrintString "Server Created Successfully")
          (Game|OpenLevel(byName) "PVP_Map" true "?listen"))
        (:OnFailure
          (|DestroySession (Game|GetPlayerController 0)
            (:OnSuccess
              (goto _label_2))))))))