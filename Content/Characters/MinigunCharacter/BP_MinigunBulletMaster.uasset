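; Base minigun bullet projectile that sets its velocity and plays a gunshot sound on spawn.
; On mesh overlap with a damageable non-instigator, it applies a GAS gameplay effect, reports an AI damage event and destroys itself.
; In co-op game mode, only actors on another team, checked through BPI_TeamCommunication, take the effect.
; Blocking hits destroy it; the gameplay-event calls to the instigator are disconnected.
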(event OnComponentBeginOverlap(Mesh)
  (params (OverlappedComponent :type Primitive%20Component%20Object%20Reference) (OtherActor :type Actor%20Object%20Reference) (OtherComp :type Primitive%20Component%20Object%20Reference) (OtherBodyIndex :type Integer) (bFromSweep :type Boolean) (SweepResult :type Hit%20Result%20Structure%20%28by%20ref%29))
  (if (!= OtherActor (Game|GetInstigator))
    (if (Variables|/Script/Engine.Actor|GetbCanBeDamaged OtherActor)
      (bind _returnvalue (Game|GetCurrentLevelName true))
      (if (.bSuccess (Utilities|Casting|CastToBP_Gamemode_Coop (Game|GetGameMode)))
        (Utilities|IsEnemy OtherActor
          (:true
            _)))
      (GameplayEffects|ApplyGameplayEffectToSelf :self (Ability|GetAbilitySystemComponent OtherActor) :GameplayEffectClass (Variables|Default|GetGameplay%20Effect%20Class) :Level 1.0)
      (Class|AISenseDamage|ReportDamageEvent OtherActor (Game|GetInstigator) 1e+01 (Transformation|GetActorLocation))
      (Actor|DestroyActor))))

(event OnComponentHit(Mesh)
  (params (HitComponent :type Primitive%20Component%20Object%20Reference) (OtherActor :type Actor%20Object%20Reference) (OtherComp :type Primitive%20Component%20Object%20Reference) (NormalImpulse :type Vector :default "0, 0, 0") (Hit :type Hit%20Result%20Structure%20%28by%20ref%29))
  (Actor|DestroyActor))

(event EventBeginPlay
  (Variables|/Script/Engine.MovementComponent|SetVelocity (Variables|Default|GetProjectileMovement) (Variables|Default|GetVelocity))
  (Audio|PlaySoundatLocation "/Game/Characters/MinigunCharacter/Sounds/S_NegevShotSingle.S_NegevShotSingle" (Transformation|GetActorLocation) "0, 0, 0" 1.0 1.0 0.0 0 0 self))

(fn ConstructionScript)

(fn PrintAttribute
  (params (PrintToScreen :type Boolean) (Actor :type Actor%20Object%20Reference) (Attribute :type Gameplay%20Attribute%20Structure))
  (Development|PrintString (Utilities|String|ToString(Float) (.ReturnValue (Ability|Attribute|GetFloatAttributefromAbilitySystemComponent (Ability|GetAbilitySystemComponent Actor) Attribute))) PrintToScreen))

(fn SendGameplayEvent
  (params (EventTag :type Gameplay%20Tag%20Structure) (TargetActor :type Actor%20Object%20Reference))
  (bind _returnvalue (Game|GetInstigator))
  (Ability|SendGameplayEventtoActor _returnvalue EventTag (Utilities|Struct|MakeGameplayEventData "(TagName=\"\")" _returnvalue TargetActor 0 0 "()" "(GameplayTags=)" "(GameplayTags=)" 0.0 (Ability|TargetData|AbilityTargetDatafromActor TargetActor))))