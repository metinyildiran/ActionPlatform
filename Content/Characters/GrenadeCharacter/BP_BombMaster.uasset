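; Base bomb projectile for the grenade character that launches at a set velocity with a random spin and fuse sparks.
; Sphere overlap with a damageable non-instigator applies a GAS damage effect, reports damage, launches characters upward, then explodes.
; In co-op mode only actors on another team, checked via team interface, are affected.
; Mesh hits only explode with sound and particles; gameplay-event sends are left unwired.
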(event OnComponentHit(Mesh)
  (params (HitComponent :type Primitive%20Component%20Object%20Reference) (OtherActor :type Actor%20Object%20Reference) (OtherComp :type Primitive%20Component%20Object%20Reference) (NormalImpulse :type Vector :default "0, 0, 0") (Hit :type Hit%20Result%20Structure%20%28by%20ref%29))
  (Utilities|Destroy "/Game/Characters/GrenadeCharacter/Sounds/S_Bomb.S_Bomb" "/Game/Characters/GrenadeCharacter/Particles/P_Explosion.P_Explosion" "0.500000,0.500000,0.500000"))

(event OnComponentBeginOverlap(Sphere)
  (params (OverlappedComponent :type Primitive%20Component%20Object%20Reference) (OtherActor :type Actor%20Object%20Reference) (OtherComp :type Primitive%20Component%20Object%20Reference) (OtherBodyIndex :type Integer) (bFromSweep :type Boolean) (SweepResult :type Hit%20Result%20Structure%20%28by%20ref%29))
  (if (!= OtherActor (Game|GetInstigator))
    (if (Variables|/Script/Engine.Actor|GetbCanBeDamaged OtherActor)
      (bind _returnvalue (Game|GetCurrentLevelName true))
      (if (.bSuccess (Utilities|Casting|CastToBP_Gamemode_Coop (Game|GetGameMode)))
        (Utilities|IsEnemy OtherActor
          (:true
            _)))
      (GameplayEffects|ApplyGameplayEffectToSelf :self (Ability|GetAbilitySystemComponent OtherActor) :GameplayEffectClass "/Game/Characters/GrenadeCharacter/GAS/Effects/GE_BombDamage.GE_BombDamage_C" :Level 1.0)
      (Class|AISenseDamage|ReportDamageEvent OtherActor (Game|GetInstigator) 1e+01 (Transformation|GetActorLocation))
      (bind _ascharacter (Utilities|Casting|CastToCharacter OtherActor))
      (Utilities|IsValid _ascharacter
        (:Is%20Valid
          (Character|LaunchCharacter _ascharacter "0, 0,700.000000" true true))
        (:Is%20Not%20Valid
          _))
      (Utilities|Destroy "/Game/Characters/GrenadeCharacter/Sounds/S_Bomb.S_Bomb" "/Game/Characters/GrenadeCharacter/Particles/P_Explosion.P_Explosion" "0.500000,0.500000,0.500000"))))

(event EventBeginPlay
  (bind _returnvalue (Math|Random|RandomFloatinRange 0.0 3.6e+02))
  (Variables|/Script/Engine.MovementComponent|SetVelocity (Variables|Default|GetProjectileMovement) (Variables|Default|GetVelocity))
  (Effects|SpawnEmitterAttached "/Game/Characters/GrenadeCharacter/Particles/P_BombSparks.P_BombSparks" (Variables|Default|GetMesh) "Fuse")
  (Variables|/Script/Engine.RotatingMovementComponent|SetRotationRate (Variables|Default|GetRotatingMovement) (Math|Rotator|MakeRotator _returnvalue _returnvalue 0.0)))

(fn ConstructionScript
  (|CallParentFunction))

(fn PrintAttribute
  (params (PrintToScreen :type Boolean) (Actor :type Actor%20Object%20Reference) (Attribute :type Gameplay%20Attribute%20Structure))
  (Development|PrintString (Utilities|String|ToString(Float) (.ReturnValue (Ability|Attribute|GetFloatAttributefromAbilitySystemComponent (Ability|GetAbilitySystemComponent Actor) Attribute))) PrintToScreen))

(fn SendGameplayEvent
  (params (EventTag :type Gameplay%20Tag%20Structure) (TargetActor :type Actor%20Object%20Reference))
  (bind _returnvalue (Game|GetInstigator))
  (Ability|SendGameplayEventtoActor _returnvalue EventTag (Utilities|Struct|MakeGameplayEventData "(TagName=\"\")" _returnvalue TargetActor 0 0 "()" "(GameplayTags=)" "(GameplayTags=)" 0.0 (Ability|TargetData|AbilityTargetDatafromActor TargetActor))))