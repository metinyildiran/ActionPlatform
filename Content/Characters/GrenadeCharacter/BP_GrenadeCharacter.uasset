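; Character Blueprint that previews a grenade throw arc, with mouse wheel input sending a clamped throw distance through SR_SetDistance.
; BeginPlay creates a spline and end-point actor, which Tick updates through OC_DrawPredictionMesh from a projectile path prediction.
; Spline mesh segments are destroyed and rebuilt every tick along that path, and the end-point marker shows only on a hit.
; Cursor-based distance and facing logic is present but disconnected.
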(event Custom|SR_SetDistance
  (params (GrenadeDistance :type Float%20%28single-precision%29))
  ;[0 0.1188 1] Draw Grenade Prediction Mesh
  (Variables|Default|SetGrenadeDistance GrenadeDistance))

(event Custom|OC_DrawPredictionMesh
  ;[0 0.1188 1] Draw Grenade Prediction Mesh
  (Throwing|DrawPredictionSpline))

(event EventTick
  (params (DeltaSeconds :type Float%20%28single-precision%29))
  ;[0 0.1188 1] Draw Grenade Prediction Mesh
  (CallFunction|OCDrawPredictionMesh))

(event EventBeginPlay
  (|CallParentFunction)
  (Throwing|CreatePredictionSpline))

(event Input|KeyboardEvents|A
  (params (Key :type Key%20Structure))
  ;[1 1 1] // Mouse Location On Screen
)

(event Input|KeyboardEvents|D
  (params (Key :type Key%20Structure))
  ;[1 1 1] // Mouse Location On Screen
)

(event Input|MouseEvents|MouseWheelUp
  (params (Key :type Key%20Structure))
  ;[0 0.1188 1] Draw Grenade Prediction Mesh
  (:Pressed
    (CallFunction|SRSetDistance (Math|Float|Clamp(Float) (+ (Variables|Default|GetGrenadeDistance) 7e+01) 2e+02 7e+02))))

(event Input|MouseEvents|MouseWheelDown
  (params (Key :type Key%20Structure))
  ;[0 0.1188 1] Draw Grenade Prediction Mesh
  (:Pressed
    (CallFunction|SRSetDistance (Math|Float|Clamp(Float) (- (Variables|Default|GetGrenadeDistance) 7e+01) 2e+02 7e+02))))

(fn ConstructionScript)

(fn CreatePredictionSpline
  (bind _returnvalue (AddComponent|AddSplineComponent false))
  (Variables|Throwing|SetPredictionSpline _returnvalue)
  (bind _returnvalue_2 (Game|SpawnActorfromClass "/Game/Characters/GrenadeCharacter/BP_PredictionEndPoint.BP_PredictionEndPoint_C" (Math|Transform|MakeTransform "0, 0, 0" "0, 0, 0" "0.400000,0.400000,0.400000") "Undefined" 0 0))
  (bind _output_get (Variables|Throwing|SetPredictionEndPoint _returnvalue_2))
  (Rendering|SetActorHiddenInGame _output_get false))

(fn DestroyPredictionSpline
  (bind _predictionspline (Variables|Throwing|GetPredictionSpline)
    (:then
      (Components|DestroyComponent _predictionspline)
      (Variables|Throwing|SetPredictionSpline 0)
      (Throwing|DestroyPredictionMeshes)
      (bind _predictionendpoint (Variables|Throwing|GetPredictionEndPoint)
        (:then
          (Actor|DestroyActor _predictionendpoint)
          (Variables|Throwing|SetPredictionEndPoint 0))
        (:else)))
    (:else)))

(fn DrawPredictionSpline
  (bind _predictionendpoint (Variables|Throwing|GetPredictionEndPoint))
  (Utilities|IsPredictionSplineValid?
    (:Is%20Valid
      (Utilities|FlowControl|Sequence
        (:then_0
          (bind (_outhit _outpathpositions _outlasttracedestination _returnvalue) (Class|GameplayStatics|BlueprintPredictProjectilePathbyTraceChannel (Utilities|ThrowLocation) (Utilities|ThrowVelocity) true 25.0 "ECC_Pawn" false (Utilities|Array|MakeArray self) "None"))
          (if _returnvalue
            (Rendering|SetActorHiddenInGame _predictionendpoint false)
            (Transformation|SetActorLocation (Variables|Throwing|GetPredictionEndPoint) (.ImpactPoint (Collision|BreakHitResult _outhit)) false true)
            (else
              (Rendering|SetActorHiddenInGame _predictionendpoint true)))
          (Spline|SetSplinePoints (Variables|Throwing|GetPredictionSpline) _outpathpositions "World" true)
          (Throwing|DestroyPredictionMeshes))
        (:then_1
          ;[1 1 1] Meshes Along Spline
          (for _index (range 0 (Math|Float|Truncate (/ (Spline|GetSplineLength (Variables|Throwing|GetPredictionSpline)) 1e+02)))
            (LocalVariables|SetIndex _index)
            (bind _returnvalue_2 (AddComponent|AddSplineMeshComponent true))
            (Utilities|Array|Add (Variables|Throwing|GetPredictionSplineMeshes) _returnvalue_2)
            (SplineMesh|SetStartandEnd _returnvalue_2 (Spline|GetLocationatDistanceAlongSpline (Variables|Throwing|GetPredictionSpline) (* (LocalVariables|GetIndex) 1e+02) "World") (Math|Vector|ClampVectorSize (Spline|GetTangentatDistanceAlongSpline (Variables|Throwing|GetPredictionSpline) (* (LocalVariables|GetIndex) 1e+02) "World") 0.0 1e+02) (Spline|GetLocationatDistanceAlongSpline (Variables|Throwing|GetPredictionSpline) (* (+ (LocalVariables|GetIndex) 1) 1e+02) "World") (Math|Vector|ClampVectorSize (Spline|GetTangentatDistanceAlongSpline (Variables|Throwing|GetPredictionSpline) (* (+ (LocalVariables|GetIndex) 1) 1e+02) "World") 0.0 1e+02) true :!class /Script/Engine.SplineMeshComponent)))))))

(fn DestroyPredictionMeshes
  (bind _predictionsplinemeshes (Variables|Throwing|GetPredictionSplineMeshes))
  (for _array_element _predictionsplinemeshes
    (Components|DestroyComponent _array_element))
  (Utilities|Array|Clear _predictionsplinemeshes))