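; Base thrown mine for the grenade character that launches via ProjectileMovement, detonates other mines of its class on spawn and simulates physics on hit.
; DetectionRadius triggers it on damageable non-instigator actors, limited to other teams via BPI_TeamCommunication in co-op mode.
; Detonation applies GE_MineDamage through GAS to characters in DamageRadius and reports damage events to AI perception.
; It then plays explosion effects and destroys itself.
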(event OnComponentBeginOverlap(DetectionRadius)
  (params (OverlappedComponent :type Primitive%20Component%20Object%20Reference) (OtherActor :type Actor%20Object%20Reference) (OtherComp :type Primitive%20Component%20Object%20Reference) (OtherBodyIndex :type Integer) (bFromSweep :type Boolean) (SweepResult :type Hit%20Result%20Structure%20%28by%20ref%29))
  (if (!= OtherActor (Game|GetInstigator))
    (if (Variables|/Script/Engine.Actor|GetbCanBeDamaged OtherActor)
      (bind _returnvalue (Game|GetCurrentLevelName true))
      (if (.bSuccess (Utilities|Casting|CastToBP_Gamemode_Coop (Game|GetGameMode)))
        (Utilities|IsEnemy OtherActor
          (:true
            _)))
      (for _array_element (Collision|GetOverlappingActors (Variables|Default|GetDamageRadius) "/Script/Engine.Character" :!class /Script/Engine.PrimitiveComponent)
        (GameplayEffects|ApplyGameplayEffectToSelf :self (Ability|GetAbilitySystemComponent _array_element) :GameplayEffectClass "/Game/Characters/GrenadeCharacter/GAS/Effects/GE_MineDamage.GE_MineDamage_C" :Level 1.0)
        (Class|AISenseDamage|ReportDamageEvent 0 (Game|GetInstigator) 1e+01 (Transformation|GetActorLocation)))
      (Utilities|Destroy "/Game/Characters/GrenadeCharacter/Sounds/S_Bomb.S_Bomb" "/Game/Characters/GrenadeCharacter/Particles/P_Explosion.P_Explosion" "0.500000,0.500000,0.500000"))))

(event OnComponentHit(Mesh)
  (params (HitComponent :type Primitive%20Component%20Object%20Reference) (OtherActor :type Actor%20Object%20Reference) (OtherComp :type Primitive%20Component%20Object%20Reference) (NormalImpulse :type Vector :default "0, 0, 0") (Hit :type Hit%20Result%20Structure%20%28by%20ref%29))
  (Physics|SetSimulatePhysics (Variables|Default|GetMesh) true))

(event Custom|Detonate
  (for _array_element (Collision|GetOverlappingActors (Variables|Default|GetDamageRadius) "/Script/Engine.Character" :!class /Script/Engine.PrimitiveComponent)
    (GameplayEffects|ApplyGameplayEffectToSelf :self (Ability|GetAbilitySystemComponent _array_element) :GameplayEffectClass "/Game/Characters/GrenadeCharacter/GAS/Effects/GE_MineDamage.GE_MineDamage_C" :Level 1.0)
    (Class|AISenseDamage|ReportDamageEvent 0 (Game|GetInstigator) 1e+01 (Transformation|GetActorLocation)))
  (Utilities|Destroy "/Game/Characters/GrenadeCharacter/Sounds/S_Bomb.S_Bomb" "/Game/Characters/GrenadeCharacter/Particles/P_Explosion.P_Explosion" "0.500000,0.500000,0.500000"))

(event EventBeginPlay
  (Variables|/Script/Engine.MovementComponent|SetVelocity (Variables|Default|GetProjectileMovement) (Variables|Default|GetVelocity))
  (bind _asbp_mine_master (Utilities|Casting|CastToBP_MineMasterClass (Variables|Default|GetMineClass)))
  (bind _outactors (Actor|GetAllActorsOfClass _asbp_mine_master))
  (for _array_element _outactors
    (if (!= _array_element self)
      (CallFunction|Detonate _array_element))))

(fn ConstructionScript)