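; Base enemy AI character that runs an assigned behavior tree and reports its destruction to the game mode for wave spawning.
; BeginPlay grants GAS abilities and applies health and damage debuffs from its owning spawn point.
; Server-side sight perception sets the blackboard TargetActor, team-checking non-player characters in co-op.
; Fire triggers the highest-numbered special off cooldown, and downward traces launch the character when stuck on edges.
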(event OnTargetPerceptionUpdated(AIPerception)
  (params (Actor :type Actor%20Object%20Reference) (Stimulus :type AI%20Stimulus%20Structure))
  ;[1 1 1] //
)

(event OnPerceptionUpdated(AIPerception)
  (params (UpdatedActors :type Array%20of%20Actor%20Object%20References))
  ;[0 0.995 0] AI Perception
  (if (Variables|Default|GetIsBehaviorTreeSet)
    (Networking|SwitchHasAuthority
      (:Authority
        (for _array_element UpdatedActors
          (bind _asbp_master_character (Utilities|Casting|CastToBP_MasterCharacter _array_element)
            (:then
              (bind _info (Class|AIPerceptionComponent|GetActorsPerception (Variables|Default|GetAIPerception) _array_element))
              (for _array_element_2 (.lastsensedstimuli _info)
                (bind _returnvalue (Class|AIPerceptionSystem|GetSenseClassforStimulus _array_element_2))
                (if (.bSuccessfullySensed (Utilities|Struct|BreakAIStimulus _array_element_2))
                  (switch string (Utilities|GetClassDisplayName _returnvalue)
                    (:AISense_Sight
                      (AI|Components|Blackboard|SetValueasObject (Class|MasterEnemyAI|GetBlackboard) (Utilities|Name|MakeLiteralName "TargetActor") _asbp_master_character))))))
            (:CastFailed
              (bind _asbase_character (Utilities|Casting|CastToBaseCharacter _array_element))
              (bind _returnvalue_2 (Game|GetCurrentLevelName true))
              (if (.bSuccess (Utilities|Casting|CastToBP_Gamemode_Coop (Game|GetGameMode)))
                (Utilities|IsEnemy _array_element
                  (:true
                    _)))
              (bind _info_2 (Class|AIPerceptionComponent|GetActorsPerception (Variables|Default|GetAIPerception) _array_element))
              (for _array_element_3 (.lastsensedstimuli _info_2)
                (bind _returnvalue_3 (Class|AIPerceptionSystem|GetSenseClassforStimulus _array_element_3))
                (if (.bSuccessfullySensed (Utilities|Struct|BreakAIStimulus _array_element_3))
                  (switch string (Utilities|GetClassDisplayName _returnvalue_3)
                    (:AISense_Sight
                      (AI|Components|Blackboard|SetValueasObject (Class|MasterEnemyAI|GetBlackboard) (Utilities|Name|MakeLiteralName "TargetActor") _asbase_character))))))))))))

(event Custom|SR_Fire
  ;[1 0 0] Fire
  (if (Variables|Default|GetCanUseSpecial3)
    (Class|MasterCharacter|ActivateAbility 2)
    (Variables|Default|SetCanUseSpecial3 false)
    (Utilities|FlowControl|Delay (Variables|Default|GetSpecial3Cooldown))
    (Variables|Default|SetCanUseSpecial3 true)
    (elif (Variables|Default|GetCanUseSpecial2)
      (Class|MasterCharacter|ActivateAbility 1)
      (Variables|Default|SetCanUseSpecial2 false)
      (Utilities|FlowControl|Delay (Variables|Default|GetSpecial2Cooldown))
      (Variables|Default|SetCanUseSpecial2 true)
      (elif (Variables|Default|GetCanUseSpecial1)
        (Class|MasterCharacter|ActivateAbility)
        (Variables|Default|SetCanUseSpecial1 false)
        (Utilities|FlowControl|Delay (Variables|Default|GetSpecial1Cooldown))
        (Variables|Default|SetCanUseSpecial1 true)))))

(event Custom|SetBehaviorTree
  (params (BTAsset :type Behavior%20Tree%20Object%20Reference))
  (bind _self self)
  (bind _returnvalue (AI|GetAIController _self))
  ;[1 1 0] Behavior Tree Setup
  (Utilities|FlowControl|Delay 1.0)
  (Utilities|IsValid _returnvalue
    (:Is%20Valid
      (AI|RunBehaviorTree _returnvalue BTAsset)
      (AI|Components|Blackboard|SetValueasBool (Class|MasterEnemyAI|GetBlackboard) (Utilities|Name|MakeLiteralName "IsSelfAlive") true)
      (Variables|Default|SetIsBehaviorTreeSet true))))

(event Custom|Fire
  ;[1 0 0] Fire
  (CallFunction|SRFire))

(event Custom|JumpIfItIsStuckOnEdge
  (bind _returnvalue (Math|Float|MakeLiteralFloat 1.2e+02))
  (bind _ishit (Utilities|DrawLineTrace "0,42.000000,0" _returnvalue))
  (bind _ishit_2 (Utilities|DrawLineTrace "0,-42.000000,0" _returnvalue))
  (bind _ishit_3 (Utilities|DrawLineTrace "42.000000,0.000000,0" _returnvalue))
  (bind _ishit_4 (Utilities|DrawLineTrace "-42.000000,0.000000,0" _returnvalue))
  (if (and (Math|Boolean|NANDBoolean _ishit _ishit_2 _ishit_3 _ishit_4) (== (Math|Vector|VectorLength (Transformation|GetVelocity)) 0.0))
    (Character|LaunchCharacter (Math|Vector|MakeVector 0.0 (* (.y (Transformation|GetActorForwardVector)) 3.5e+02) 3.5e+02) true true)))

(event EventBeginPlay
  (CallFunction|InitializeAbilities (Variables|Default|GetAbilityList))
  (bind _asbp_spawn_point (Utilities|Casting|CastToBP_SpawnPoint (Components|GetOwner)))
  (Utilities|FlowControl|Delay 1.0)
  (GameplayEffects|ApplyGameplayEffectToSelf :self (Variables|Default|GetAbilitySystemComponent) :GameplayEffectClass (Variables|/Game/SideScrollerBP/Blueprints/Wave/BP_SpawnPoint.BP_SpawnPoint_C|GetHealth%20Debuff _asbp_spawn_point) :Level 1.0)
  (GameplayEffects|ApplyGameplayEffectToSelf :self (Variables|Default|GetAbilitySystemComponent) :GameplayEffectClass (Variables|/Game/SideScrollerBP/Blueprints/Wave/BP_SpawnPoint.BP_SpawnPoint_C|GetDamage%20Debuff _asbp_spawn_point) :Level 1.0))

(event EventTick
  (params (DeltaSeconds :type Float%20%28single-precision%29))
  ;[1 0 0] Debug
)

(event EventDestroyed
  ;[0 0.134 1] For wave spawning
  (Class|BPIGameMode|EnemyHasDied(Message) (Game|GetGameMode)))

(fn ConstructionScript
  (Transformation|AttachComponentToComponent (Variables|Default|GetMask) (Variables|Character|GetMesh) "head_001Socket" "KeepRelative" "KeepRelative" "KeepRelative" true))

(fn InitializeAbilities
  (params (Array :type Array%20of%20Gameplay%20Ability%20Class%20References))
  (for (_array_element _array_index) Array
    (Class|MasterCharacter|GrantAbility _array_element 1 _array_index)))

(fn PrintAttribute
  (params (Actor%28self%29 :type Actor%20Object%20Reference) (Attribute :type Gameplay%20Attribute%20Structure) (AttributeName :type String) (Duration :type Float%20%28single-precision%29))
  (bind _self self)
  (Utilities|IsValid Actor%28self%29
    (:Is%20Valid
      (Development|PrintString (Utilities|String|Append (Utilities|GetObjectName Actor%28self%29) "->" AttributeName ":" (Utilities|String|ToString(Float) (.ReturnValue (Ability|Attribute|GetFloatAttributefromAbilitySystemComponent (Ability|GetAbilitySystemComponent Actor%28self%29) Attribute)))) true true "(R=1.000000,G=0.000000,B=0.000000,A=1.000000)" Duration))
    (:Is%20Not%20Valid
      (Development|PrintString (Utilities|String|Append (Utilities|GetObjectName _self) "->" AttributeName ":" (Utilities|String|ToString(Float) (.ReturnValue (Ability|Attribute|GetFloatAttributefromAbilitySystemComponent (Ability|GetAbilitySystemComponent _self) Attribute)))) true true "(R=1.000000,G=0.000000,B=0.000000,A=1.000000)" Duration))))

(fn GetTeamNum
  (return (Variables|Default|GetTeamNum)))